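; Paper2D patrolling enemy that walks along platforms and is destroyed, with a sound, when a bullet overlaps its box.
; Each tick it moves along its forward vector and traces down from an arrow component, rotating 180 degrees when no ground is found.
; It also records horizontal direction, which is never read here, and sets the same flipbook whether moving or idle.
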(event OnComponentBeginOverlap(Box)
  (params (OverlappedComponent :type Primitive%20Component%20Object%20Reference) (OtherActor :type Actor%20Object%20Reference) (OtherComp :type Primitive%20Component%20Object%20Reference) (OtherBodyIndex :type Integer) (bFromSweep :type Boolean) (SweepResult :type Hit%20Result%20Structure%20%28by%20ref%29))
  (Utilities|Casting|CastToBullet_BP OtherActor)
  (Audio|PlaySound2D "/Game/Asset4_Audio/CollectCoin_Sound.CollectCoin_Sound" 1.0 1.0 0.0 0 0)
  (Actor|DestroyActor))

(event Custom|CheckDirection
  (if (> (.x (Transformation|GetVelocity)) 0.0)
    (Variables|Default|SetbisMoveRight true)
    (elif (< (.x (Transformation|GetVelocity)) 0.0)
      (Variables|Default|SetbisMoveRight false))))

(event Custom|Movement
  (Pawn|Input|AddMovementInput (Transformation|GetActorForwardVector) (Variables|Default|GetScale%20Value) false))

(event Custom|UpdateAnimation
  (Sprite|SetFlipbook (Variables|Default|GetPaperFlipbook) (select (> (Math|Vector|VectorLength (Transformation|GetVelocity)) 0.0) "/Game/Asset3_Flipbook/EnemyFlipbook.EnemyFlipbook" "/Game/Asset3_Flipbook/EnemyFlipbook.EnemyFlipbook")))

(event Custom|Turn%20Char
  (Transformation|SetActorRotation (Math|Rotator|CombineRotators (Transformation|GetActorRotation) "0.000000,180.000000,0.000000")))

(event Custom|EdgeCheck
  (bind _arrow_check (Variables|Default|GetArrow_Check))
  (bind _outhit (Collision|LineTraceByChannel (Transformation|GetWorldLocation _arrow_check) (- (Transformation|GetWorldLocation _arrow_check) "0.000000,0.000000,200.000000") "TraceTypeQuery1" false 0 "None"))
  (if (not (.bBlockingHit (Collision|BreakHitResult _outhit)))
    (CallFunction|TurnChar)))

(event EventTick
  (params (DeltaSeconds :type Float%20%28single-precision%29))
  (CallFunction|Movement)
  (CallFunction|CheckDirection)
  (CallFunction|EdgeCheck)
  (CallFunction|UpdateAnimation))

(fn ConstructionScript)