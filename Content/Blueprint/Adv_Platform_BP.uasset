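; Adv_Platform_BP is a platform that the player character can land on from above and drop through.
; Overlapping the upper box turns the render component's collision on after a short delay.
; Overlapping the lower box enables input on the platform, after which pressing C turns that collision off after the same delay.
; A status flag prevents redundant toggles, and debug prints report input and collision changes.
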(event OnComponentBeginOverlap(Upper_Box)
  (params (OverlappedComponent :type Primitive%20Component%20Object%20Reference) (OtherActor :type Actor%20Object%20Reference) (OtherComp :type Primitive%20Component%20Object%20Reference) (OtherBodyIndex :type Integer) (bFromSweep :type Boolean) (SweepResult :type Hit%20Result%20Structure%20%28by%20ref%29))
  (Utilities|Casting|CastToMyCharacter OtherActor)
  (if (not (Variables|Default|GetPlatform_Collision_Status))
    (Utilities|FlowControl|Delay 0.2)
    (Collision|SetCollisionEnabled (Variables|Default|GetRenderComponent) "QueryAndPhysics")
    (Variables|Default|SetPlatform_Collision_Status true)))

(event OnComponentBeginOverlap(Lower_Box)
  (params (OverlappedComponent :type Primitive%20Component%20Object%20Reference) (OtherActor :type Actor%20Object%20Reference) (OtherComp :type Primitive%20Component%20Object%20Reference) (OtherBodyIndex :type Integer) (bFromSweep :type Boolean) (SweepResult :type Hit%20Result%20Structure%20%28by%20ref%29))
  (Utilities|Casting|CastToMyCharacter OtherActor)
  (Input|EnableInput (Game|GetPlayerController 0))
  (Development|PrintString "Enabled Input"))

(event EventBeginPlay)

(event Collision|EventActorBeginOverlap
  (params (OtherActor :type Actor%20Object%20Reference)))

(event EventTick
  (params (DeltaSeconds :type Float%20%28single-precision%29)))

(event Input|KeyboardEvents|C
  (params (Key :type Key%20Structure :default "None"))
  (:Pressed
    (Development|PrintString "Set No Collision")
    (if (Variables|Default|GetPlatform_Collision_Status)
      (Utilities|FlowControl|Delay 0.2)
      (Collision|SetCollisionEnabled (Variables|Default|GetRenderComponent) "NoCollision")
      (Variables|Default|SetPlatform_Collision_Status false))))

(fn ConstructionScript)